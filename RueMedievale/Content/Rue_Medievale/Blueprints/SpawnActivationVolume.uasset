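; Trigger volume that activates a list of referenced actors when the player enters its box and deactivates them when the player leaves.
; Actors receive Activate and Deactivate messages through BI_Activatable, and those without the interface ignore them.
; A DoOnce limits activation to the first entry until the BP_FirstPersonPlayerController reset-world event re-arms it, while deactivation fires on every exit.
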(event OnComponentBeginOverlap(Box)
  (params (OverlappedComponent :type Primitive%20Component%20Object%20Reference) (OtherActor :type Actor%20Object%20Reference) (OtherComp :type Primitive%20Component%20Object%20Reference) (OtherBodyIndex :type Integer) (bFromSweep :type Boolean) (SweepResult :type Hit%20Result%20Structure%20%28by%20ref%29))
  ;[0.15 0.15 0.15 0.5] Collision volume overlap events
  ;;[0.15 0.15 0.15 0.5] Has the player entered this volume?
  (if (== OtherActor (Game|GetPlayerCharacter 0))
    (Utilities|FlowControl|DoOnce false
      (:Completed
        (Utilities|FlowControl|Sequence
          (:then_0
            ;;[0.15 0.15 0.15 0.5] Activate each Actor referenced by this volume. Actors must implement the BI_Activatable interface, otherwise they are ignored.
            (for _array_element (Variables|Default|GetActors%20to%20Activate)
              (Class|BPIInteractable|Activate(Message) _array_element OtherActor))))))))

(event OnComponentEndOverlap(Box)
  (params (OverlappedComponent :type Primitive%20Component%20Object%20Reference) (OtherActor :type Actor%20Object%20Reference) (OtherComp :type Primitive%20Component%20Object%20Reference) (OtherBodyIndex :type Integer))
  ;[0.15 0.15 0.15 0.5] Collision volume overlap events
  ;;[0.15 0.15 0.15 0.5] Has the player left this volume?
  (if (== OtherActor (Game|GetPlayerCharacter 0))
    (Utilities|FlowControl|Sequence
      (:then_0
        ;;[0.15 0.15 0.15 0.5] Deactivate each Actor referenced by this volume. Actors must implement the BI_Activatable interface, otherwise they are ignored.
        (for _array_element (Variables|Default|GetActors%20to%20Activate)
          (Class|BPIInteractable|Deactivate(Message) _array_element OtherActor))))))

(event Custom|Reset
  ;[0.15 0.15 0.15 0.5] Collision volume overlap events
  ;;[0.15 0.15 0.15 0.5] Has the player entered this volume?
  (Utilities|FlowControl|DoOnce false) ; enters at Reset
)

(event EventBeginPlay
  (bind _asbp_first_person_player_controller (Utilities|Casting|CastToBP_FirstPersonPlayerController (Game|GetPlayerController 0)))
  (EventDispatchers|BindEventtoResetWorld _asbp_first_person_player_controller (delegate Custom|Reset)))

(fn ConstructionScript)