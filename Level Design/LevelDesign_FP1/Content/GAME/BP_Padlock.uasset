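; BP_Padlock is a lock actor that opens when a matching key item overlaps its trigger box.
; On overlap, it checks for the BPI_InspectSetup interface, casts to BP_ItemKey and compares the key's string to its own PadlockString.
; A match calls OpenDoor, which hides and disables collision on both the linked StaticmeshToOpen and the padlock, then plays an unlock sound through BPAudioPlay.
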(event OnComponentBeginOverlap(Box)
  (params (OverlappedComponent :type Primitive%20Component%20Object%20Reference) (OtherActor :type Actor%20Object%20Reference) (OtherComp :type Primitive%20Component%20Object%20Reference) (OtherBodyIndex :type Integer) (bFromSweep :type Boolean) (SweepResult :type Hit%20Result%20Structure%20%28by%20ref%29))
  (if (Utilities|DoesObjectImplementInterface OtherActor "/Game/GAME/BPI_InspectSetup.BPI_InspectSetup_C")
    (bind _asbp_item_key (Utilities|Casting|CastToBP_ItemKey OtherActor)
      (:then
        (if (Utilities|Enum|Equal(Enum) (Variables|/Game/GAME/BP_ItemKey.BP_ItemKey_C|GetkeyString _asbp_item_key) (Variables|Default|GetpadlockString))
          (CallFunction|OpenDoor)))
      (:CastFailed
        (Development|PrintString "KeyItem CAST FAILED")))))

(event EventBeginPlay)

(event Collision|EventActorBeginOverlap
  (params (OtherActor :type Actor%20Object%20Reference)))

(event EventTick
  (params (DeltaSeconds :type Float%20%28single-precision%29)))

(fn ConstructionScript)

(fn OpenDoor
  (bind _staticmeshtoopen (Variables|Default|GetstaticmeshToOpen))
  (Rendering|SetActorHiddenInGame _staticmeshtoopen true)
  (Collision|SetActorEnableCollision _staticmeshtoopen false)
  (Rendering|SetActorHiddenInGame true)
  (Collision|SetActorEnableCollision false)
  (Default|PlaySimpleSFX (Variables|Default|GetBP_AudioPlay) "/Game/GAME/AUDIO/SFX/Key/SFX_KeyUnlock.SFX_KeyUnlock" "NewEnumerator1" (Transformation|GetWorldLocation (Variables|Default|GetPadlock)) 1.0))