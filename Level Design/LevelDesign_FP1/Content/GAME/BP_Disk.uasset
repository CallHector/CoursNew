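; BP_Disk is a physical, interactable disk that stores signal data and can be inserted into and ejected from other devices.
; Its light color and intensity show empty or full, while text components display the signal's ID, frequency, location, comment and processed status.
; Insertion and ejection functions toggle state and physics, with a Tick timer gating reinsertion validity.
; Mailbox ejection ignores the mailbox's collision and launches the disk with a directed impulse.
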(event Custom|Destroy
  (Utilities|FlowControl|Delay 0.2)
  (Actor|DestroyActor))

(event EventBeginPlay
  (if (Variables|Default|GetisDiskEmpty)
    (CallFunction|SetColorDisk true)
    (else
      (CallFunction|SetColorDisk false)
      ;[1 1 1] SetupTextIfDiskNotEmpty
      (CallFunction|DiskFullBeginTextSetup)))
  (if (Utilities|IsValid (Variables|StaticMesh|GetStaticMeshSet))
    (Components|StaticMesh|SetStaticMesh (Variables|Default|GetDiskStaticMesh) (Variables|StaticMesh|GetStaticMeshSet))))

(event EventTick
  (params (DeltaSeconds :type Float%20%28single-precision%29))
  ;[1 1 1] Disk Grab After Eject Security Insertion
  (if (Variables|Default|GetGrabAfterEject)
    (if (>= (Variables|Default|GetEjectionSecurityTimer) (Variables|Default|GetEjectionSecurityDelay))
      (Variables|Default|SetEjectionSecurityTimer 0.0)
      (Variables|Default|SetInsertionValidSecurity true))
    (else
      (Variables|Default|SetEjectionSecurityTimer (+ (Variables|Default|GetEjectionSecurityTimer) DeltaSeconds)))))

(fn ConstructionScript)

(fn Interact
  (Development|PrintString "Interaction Enabled"))

(fn Insertion
  ;[1 1 1] InsertionSecurity
  (Variables|Default|SetEjectionSecurityTimer 0.0)
  (Variables|Default|SetInsertionValidSecurity false)
  (CallFunction|ActivatePhysics false)
  (Development|PrintString "Disk Being Inserted")
  (Variables|Default|SetGrabAfterEject false)
  (return))

(fn Ejection
  (Variables|Default|SetejectMode true)
  (Variables|Default|SetisInserted false))

(fn OverrideSignalData
  (params (DataToOverride :type Signal%20Data%20Structure%20Structure))
  (Variables|Default|SetSignalDataInDisk DataToOverride)
  (Variables|Default|SetisDiskEmpty false)
  (CallFunction|SetColorDisk false))

(fn EmptySignalData
  (Variables|Default|SetisDiskEmpty true)
  (CallFunction|SetColorDisk true)
  (Rendering|SetVisibility (Variables|Default|GetID_Text) false false)
  (Rendering|SetVisibility (Variables|Default|GetLoc_Text) false false)
  (Rendering|SetVisibility (Variables|Default|GetWolfheadComment_Text) false false)
  (Rendering|SetVisibility (Variables|Default|GetFreq_Text) false false)
  (Rendering|SetVisibility (Variables|Default|GetProcess_Text) false false))

(fn ActivatePhysics
  (params (activate :type Boolean))
  (Physics|SetSimulatePhysics (Variables|Default|GetDiskStaticMesh) activate))

(fn GrabinEjectMode
  (CallFunction|ActivatePhysics true)
  (Variables|Default|SetejectMode false)
  (Variables|Default|SetGrabAfterEject true))

(fn SetColorDisk
  (params (empty :type Boolean))
  (bind _pointlight (Variables|Default|GetPointLight))
  (bind _pointlight_2 (Variables|Default|GetPointLight))
  (if empty
    (Rendering|Components|Light|SetLightColor _pointlight_2 (Math|Conversions|ToLinearColor(Color) (Variables|Default|GetdiskEmptyColor)) true)
    (Rendering|Components|Light|SetIntensity _pointlight_2 2.0)
    (else
      (Rendering|Components|Light|SetLightColor _pointlight (Math|Conversions|ToLinearColor(Color) (Variables|Default|GetdiskFullColor)) true)
      (Rendering|Components|Light|SetIntensity _pointlight 7.0))))

(fn MailBoxEjection
  (params (ActorToIgnore :type Actor%20Object%20Reference) (ejectDirection :type Vector))
  (bind _mailboxejectforce (Variables|Default|GetmailBoxEjectForce))
  (if (Utilities|IsValid ActorToIgnore)
    ;[1 1 1 1 15] We Ignore the mailbox collision for the disk/object
    (Collision|IgnoreActorwhenMoving (Variables|Default|GetDiskStaticMesh) ActorToIgnore true))
  (CallFunction|ActivatePhysics true)
  (Physics|AddImpulse (Variables|Default|GetDiskStaticMesh) (* (Math|Vector|Normalize (- ejectDirection (Transformation|GetWorldLocation (Variables|Default|GetDiskStaticMesh)))) (Math|Vector|MakeVector _mailboxejectforce _mailboxejectforce _mailboxejectforce)) "None" false)
  (Variables|Default|SetisInserted false))

(fn SetIDText
  (params (ID :type String))
  (bind _id_text (Variables|Default|GetID_Text))
  (Rendering|SetVisibility _id_text true false)
  (Rendering|Components|TextRender|SetText _id_text (Utilities|Text|ToText(String) (Utilities|String|Append "ID : " ID))))

(fn SetLocText
  (params (Localisation :type String))
  (bind _loc_text (Variables|Default|GetLoc_Text))
  (Rendering|SetVisibility _loc_text true false)
  (Rendering|Components|TextRender|SetText _loc_text (Utilities|Text|ToText(String) Localisation)))

(fn SetWolfheadCommentText
  (params (WolfHeadComment :type String))
  (bind _wolfheadcomment_text (Variables|Default|GetWolfheadComment_Text))
  (Rendering|SetVisibility _wolfheadcomment_text true false)
  (Rendering|Components|TextRender|SetText _wolfheadcomment_text (Utilities|Text|ToText(String) WolfHeadComment)))

(fn DiskFullBeginTextSetup
  (bind _signaldataindisk (Variables|Default|GetSignalDataInDisk))
  (bind (_id _signalfrequency _sound _issignalactive _firstrecord _firstinsert _firstprocess _newrecord _timeofrecord _startsoundtimeofrecord _localisation) (Utilities|Struct|BreakSignalDataStructure _signaldataindisk))
  (SetText|SetIDText (Utilities|String|Append "ID : " _id))
  (SetText|SetFreqText (Utilities|String|ToString(Float) _signalfrequency))
  (SetText|SetLocText _localisation))

(fn SetFreqText
  (params (Frequency :type String))
  (bind _freq_text (Variables|Default|GetFreq_Text))
  (Rendering|SetVisibility _freq_text true false)
  (Rendering|Components|TextRender|SetText _freq_text (Utilities|Text|ToText(String) Frequency)))

(fn SetProcessedText
  (bind _process_text (Variables|Default|GetProcess_Text))
  (Rendering|SetVisibility _process_text true false)
  (Rendering|Components|TextRender|SetText _process_text (Utilities|Text|ToText(String) "PROCESSED")))

(fn GetSignal
  (return 0 "" false))