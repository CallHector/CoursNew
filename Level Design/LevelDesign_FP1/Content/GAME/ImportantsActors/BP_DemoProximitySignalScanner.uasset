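; Player-attached proximity scanner that helps track down saved signal emitters by sound and compass heading.
; Mouse wheel cycles the localised signal list; BPSignalScannerComponent resolves the selected frequency to an emitter and loads its sound.
; A repeating timer compares player facing with emitter bearing by cardinal direction and scales signal volume by distance.
; It plays neutral or good beeps within range, silences them up close, and pushes scanner state to the first-person character.
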(event Custom|StartLoop
  ;[1 1 1] Start Loop
  (Utilities|Time|SetTimerbyEvent (delegate Custom|StartLoop) 2.0 true)
  (if (Variables|Default|GetscannerEnabled)
    (if (Variables|Default|GetEmitterFound)
      ;[1 1 1] Signal Check Loop
      (CallFunction|SignalCheckLoop))))

(event Custom|MouseWheelUp
  (if (Variables|Default|GetlistenForMouseScrollInput)
    (CallFunction|SignalChanges 1.0)))

(event Custom|UpdateOrientationCorrect
  (params (isOrientationCorrect :type Boolean))
  ;[1 1 1] OrientationCorrect Scaner
  (Default|UpdateScannerInfo (Variables|Default|GetFirstPersonCharacter) false 0 false 0.0 "" false "" false isOrientationCorrect true))

(event Custom|MouseWheelDown
  (if (Variables|Default|GetlistenForMouseScrollInput)
    (CallFunction|SignalChanges -1.0)))

(event EventBeginPlay
  ;[0.2304 0.3524 1] BeginPlay
  (Transformation|AttachActorToActor (Game|GetPlayerCharacter 0) "None" "SnapToTarget" "SnapToTarget" "KeepRelative" true)
  (CallFunction|StartLoop)
  (bind _asbp_first_person_character (Utilities|Casting|CastToBP_FirstPersonCharacter (Game|GetPlayerCharacter 0))
    (:then
      (Variables|Default|SetFirstPersonCharacter _asbp_first_person_character))
    (:CastFailed
      (Development|PrintString "Error in BP_ProximitySignalScanner, the cast of the BP_FirstPersonCharacter Isn't working" true true "(R=1.000000,G=0.109946,B=0.000000,A=1.000000)"))))

(fn ConstructionScript)

(fn SignalChanges
  (params (isAdding :type Float%20%28double-precision%29))
  ;[1 0.7645 0.3118] SFX
  (Sound|FreqChangesSFX)
  ;[1 1 1] Security to prevent searching signals when none are saved
  (if (not (<= (Utilities|Array|Length (Variables|Default|GetSignalIDLocalised)) 0))
    ;[1 1 1] Is Adding?
    (if (== isAdding 1.0)
      ;[1 1 1] If 10 then -> 1
      (if (== (Variables|Default|GetsignalSavedNavigationNumber) (- (Utilities|Array|Length (Variables|Default|GetSignalIDLocalised)) 1))
        ;[1 1 1] Back to 1
        (Variables|Default|SetsignalSavedNavigationNumber 0)
        (else
          ;[1 1 1] Calcul du numéro de navigation en s'assurant qu'il ne dépassent pas le nombre de signal data sauvegardé
          (bind _output_get (Variables|Default|SetsignalSavedNavigationNumber (Math|Integer|Clamp(Integer) (+ (Variables|Default|GetsignalSavedNavigationNumber) 1) 0 (- (Utilities|Array|Length (Variables|Default|GetSignalIDLocalised)) 1))))))
      (else
        ;[1 1 1] If 1 then -> max
        (if (and (== (Variables|Default|GetsignalSavedNavigationNumber) 0) (Utilities|Array|IsNotEmpty (Variables|Default|GetSignalIDLocalised)))
          ;[1 1 1] Back to max (1 -> 10)
          (Variables|Default|SetsignalSavedNavigationNumber (- (Utilities|Array|Length (Variables|Default|GetSignalIDLocalised)) 1))
          (else
            ;[1 1 1] Calcul du numéro de navigation en s'assurant qu'il ne dépassent pas le nombre de signal data sauvegardé
            (Variables|Default|SetsignalSavedNavigationNumber (Math|Integer|Clamp(Integer) (- (Variables|Default|GetsignalSavedNavigationNumber) 1) 0 (- (Utilities|Array|Length (Variables|Default|GetSignalIDLocalised)) 1)))))))
    ;[1 1 1] debug To see the savec Number
    (Development|PrintString (Utilities|String|ToString(Integer) _output_get))
    (Variables|Default|SetSignalDataTargeted (Utilities|Array|Get(acopy) (Variables|Default|GetSignalIDLocalised) (Variables|Default|GetsignalSavedNavigationNumber)))
    ;[0 0 0] Getting Actor Emiting (not clean)
    (bind (_signaldatafound _anysignaldatafound _numberofsignalfound _signaldatamultiple _actoremitting) (Default|SearchSignalProximityScanner (Variables|Default|GetBP_SignalScannerComponent) (.signalFrequency (Utilities|Struct|BreakSignalDataStructure (Utilities|Array|Get(acopy) (Variables|Default|GetSignalIDLocalised) (Variables|Default|GetsignalSavedNavigationNumber))))))
    (if _anysignaldatafound
      (Variables|Default|SetActorEmitterTargeted _actoremitting)
      (Variables|Default|SetEmitterFound true)
      ;[1 1 1] Feedback SoundFound
      (Default|PlaySimpleSFX (Variables|Default|GetBP_AudioPlay) 0 "NewEnumerator6" (Transformation|GetWorldLocation (Variables|Default|GetAudio)) 1.0)
      (CallFunction|SetupSignal)
      (else
        (Variables|Default|SetEmitterFound false)
        (Development|PrintString "Emitter not found")
        ;[1 1 1 1 15] Small Security to set the volume to 0 when changing frequency
        (CallFunction|AdjustSignalPlaying 0.0 true)
        ;[1 1 1 1 12] Small Secuirty to set the color of the scanner ro white when we change freq
        (CallFunction|UpdateOrientationCorrect false)))
    ;[1 1 1 1 15] Player Scanner Freq Update
    (Default|UpdateScannerInfo (Variables|Default|GetFirstPersonCharacter) true (Variables|Default|GetsignalSavedNavigationNumber) (Utilities|Array|IsEmpty (Variables|Default|GetSignalIDLocalised)) (.signalFrequency (Utilities|Struct|BreakSignalDataStructure (Utilities|Array|Get(acopy) (Variables|Default|GetSignalIDLocalised) (Variables|Default|GetsignalSavedNavigationNumber)))) (.ID (Utilities|Struct|BreakSignalDataStructure (Utilities|Array|Get(acopy) (Variables|Default|GetSignalIDLocalised) (Variables|Default|GetsignalSavedNavigationNumber)))) true "" false false false)))

(fn BipSFX
  (params (bipType :type Integer))
  (LocalVariables|SetSoundPosition (Transformation|GetWorldLocation (Variables|/Script/Engine.Actor|GetRootComponent (Variables|Default|GetFirstPersonCharacter))))
  (switch int bipType
    (:0
      (Default|PlaySimpleSFX (Variables|Default|GetBP_AudioPlay) "/Game/GAME/AUDIO/SCANNER/SFX_Scan_Neutral.SFX_Scan_Neutral" "NewEnumerator1" (LocalVariables|GetSoundPosition) 1.0))
    (:1
      (Default|PlaySimpleSFX (Variables|Default|GetBP_AudioPlay) "/Game/GAME/AUDIO/SCANNER/SFX_Scan_Good1.SFX_Scan_Good1" "NewEnumerator1" (LocalVariables|GetSoundPosition) 1.0))
    (:2
      (Default|PlaySimpleSFX (Variables|Default|GetBP_AudioPlay) "/Game/GAME/AUDIO/SCANNER/SFX_Scan_Good2.SFX_Scan_Good2" "NewEnumerator1" (LocalVariables|GetSoundPosition) 1.0))
    (:3
      (Default|PlaySimpleSFX (Variables|Default|GetBP_AudioPlay) "/Game/GAME/AUDIO/SCANNER/SFX_Scan_Good3.SFX_Scan_Good3" "NewEnumerator1" (LocalVariables|GetSoundPosition) 1.0))))

(fn DistanceCheck
  (if (Variables|Default|GetEmitterFound)
    (return (/ (Math|Vector|VectorLength (- (Transformation|GetActorLocation (Variables|/Game/GAME/ImportantsActors/BP_SignalScannerComponent.BP_SignalScannerComponent_C|GetActorEmmitingFound (Variables|Default|GetBP_SignalScannerComponent))) (Transformation|GetWorldLocation (Variables|/Script/Engine.Character|GetCapsuleComponent (Game|GetPlayerCharacter 0))))) 1e+02))))

(fn ShowScanner
  (Variables|Default|SetscannerEnabled true)
  (Development|PrintString "ScannerEnabled")
  (Sound|ShowScannerSFX)
  (Default|ShowScanner (Variables|Default|GetFirstPersonCharacter))
  (CallFunction|SignalChanges 0.0))

(fn HideScanner
  (Variables|Default|SetscannerEnabled false)
  (Development|PrintString "ScannerDisabled")
  (Sound|HideScannerSFX)
  (Default|HideScanner (Variables|Default|GetFirstPersonCharacter))
  (CallFunction|AdjustSignalPlaying 0.0 true))

(fn ListenforMouseScroll
  (params (listenForMouseScrollInput :type Boolean))
  (Variables|Default|SetlistenForMouseScrollInput listenForMouseScrollInput))

(fn FreqChangesSFX
  (Default|PlaySimpleSFX (Variables|Default|GetBP_AudioPlay) 0 "NewEnumerator2" (Transformation|GetWorldLocation (Variables|/Script/Engine.Character|GetCapsuleComponent (Game|GetPlayerCharacter 0))) 1.0))

(fn ShowScannerSFX
  (Default|PlaySimpleSFX (Variables|Default|GetBP_AudioPlay) "/Engine/VREditor/Sounds/UI/Floating_UI_Open-002.Floating_UI_Open-002" "NewEnumerator1" (Transformation|GetWorldLocation (Variables|/Script/Engine.Character|GetCapsuleComponent (Variables|Default|GetFirstPersonCharacter))) 1.0))

(fn HideScannerSFX
  (Default|PlaySimpleSFX (Variables|Default|GetBP_AudioPlay) "/Engine/VREditor/Sounds/UI/Floating_UI_Close-002.Floating_UI_Close-002" "NewEnumerator1" (Transformation|GetWorldLocation (Variables|/Script/Engine.Character|GetCapsuleComponent (Variables|Default|GetFirstPersonCharacter))) 1.0))

(fn AdjustSignalPlaying
  (params (distance :type Float%20%28double-precision%29) (disableSignal :type Boolean))
  (if disableSignal
    (Audio|Components|Audio|AdjustVolume (Variables|Default|GetAudio) 0.0 0.0 "Linear" :!class /Script/Engine.AudioComponent)
    (else
      (Audio|Components|Audio|AdjustVolume (Variables|Default|GetAudio) 0.0 (Math|Float|Lerp 0.7 0.0001 (/ (Math|Float|Clamp(Float) (- distance 1.0) 0.0 (Variables|Default|GetdistanceMinimumToHearSignal)) (Variables|Default|GetdistanceMinimumToHearSignal))) "Linear" :!class /Script/Engine.AudioComponent))))

(fn SetupSignal
  (bind _signaldatatargeted (Variables|Default|GetSignalDataTargeted))
  (Variables|Default|SetSignalDataPlaying _signaldatatargeted)
  (Audio|Components|Audio|SetSound (Variables|Default|GetAudio) (.sound (Utilities|Struct|BreakSignalDataStructure _signaldatatargeted)))
  (Audio|Components|Audio|Play (Variables|Default|GetAudio) 0.0)
  (Audio|Components|Audio|AdjustVolume (Variables|Default|GetAudio) 0.0 1e-05 "Linear" :!class /Script/Engine.AudioComponent))

(fn SignalCheckLoop
  (bind _distance (CallFunction|DistanceCheck))
  (LocalVariables|SetdistanceToSignal _distance)
  ;[1 0.6609 0.9011] Return Correct Orientation Or Not
  ;;[1 1 1] Player - Object Orientation
  (bind (_cardinaldirectionoutput _bearingnumbersoutput) (Default|ReturnBearingCardinalInfo (Variables|Default|GetBP_SignalScannerComponent) (Transformation|GetWorldLocation (Variables|/Script/Engine.Character|GetCapsuleComponent (Variables|Default|GetFirstPersonCharacter))) (Transformation|GetWorldLocation (Variables|/Game/GAME/BP_ItemTransmitting.BP_ItemTransmitting_C|GetStaticMesh (Variables|Default|GetActorEmitterTargeted)))))
  ;;[1 1 1] Player Camera Orientation
  (bind (_cardinaldirecton _bearingnumber) (Default|ReturnOrientation (Variables|Default|GetFirstPersonCharacter)))
  (bind _output_get (LocalVariables|SetOrientationCorrect (Utilities|Enum|Equal(Enum) _cardinaldirecton _cardinaldirectionoutput)))
  (CallFunction|UpdateOrientationCorrect _output_get)
  ;[1 1 1] Adjust Signal Playing
  (CallFunction|AdjustSignalPlaying (LocalVariables|GetdistanceToSignal) false)
  ;[1 1 1] Distance Check
  ;;[1 1 1 1 12] So Close that the Bip Stop and we hear the signal only
  (if (not (<= (LocalVariables|GetdistanceToSignal) (Variables|Default|GetdistanceStopBipNoise)))
    ;;[1 1 1 1 12] Close enough to have the Bip Sound?
    (if (<= (LocalVariables|GetdistanceToSignal) (Variables|Default|GetdistanceMinimumToHaveSignalDetection))
      (if (LocalVariables|GetOrientationCorrect)
        (CallFunction|BipSFX 1)
        (else
          (CallFunction|BipSFX))))))

(fn AddLocalisedSignal
  (params (SignalDataLocalised :type Signal%20Data%20Structure%20Structure))
  (bind (_id _signalfrequency _sound _issignalactive _firstrecord _firstinsert _firstprocess _newrecord _timeofrecord _startsoundtimeofrecord _localisation) (Utilities|Struct|BreakSignalDataStructure SignalDataLocalised))
  (bind _signalidlocalised (Variables|Default|GetSignalIDLocalised))
  (Utilities|Array|SetArrayElem _signalidlocalised (Utilities|Array|Length _signalidlocalised) SignalDataLocalised true)
  (Development|PrintString (Utilities|String|Append _id " = LOCALISED" " + " _localisation))
  ;[1 1 1] Add signal saved (to keep track of how many signal are localised)
  (Default|AddNewSignalLocalised (Variables|Default|GetFirstPersonCharacter)))