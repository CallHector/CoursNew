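; Mailbox station where the player submits signal disks to Wolfhead for judgement and later gets them back with comments.
; Box overlap stores valid disks, with a flag and short delay blocking duplicate triggers; Full Drop interaction ejects them.
; The lever grades each disk by signal ID through empty, processed and location checks, writing comments and emptying successful disks.
; A repeating timer ejects all graded disks, accepted or rejected, after a delivery sound.
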(event OnComponentBeginOverlap(Box)
  (params (OverlappedComponent :type Primitive%20Component%20Object%20Reference) (OtherActor :type Actor%20Object%20Reference) (OtherComp :type Primitive%20Component%20Object%20Reference) (OtherBodyIndex :type Integer) (bFromSweep :type Boolean) (SweepResult :type Hit%20Result%20Structure%20%28by%20ref%29))
  (bind _bp_diskinsertionlogic (Variables|Default|GetBP_DiskInsertionLogic))
  (bind _disktoinsertref (Variables|/Game/GAME/ImportantsActors/BP_DiskInsertionLogic.BP_DiskInsertionLogic_C|GetDiskToInsertRef _bp_diskinsertionlogic))
  ;[1 1 1] Disk Insert Main Logic
  ;;[1 1 1] Security to prevent the insertion to be triggered twice
  (if (Variables|DiskLogic|GetInsertionComplete)
    (bind _actorvalidforinsertion (Default|IsInsertionValid _bp_diskinsertionlogic OtherActor))
    (if _actorvalidforinsertion
      (if (Variables|DiskLogic|GetInsertionComplete)
        (if (not (Variables|/Game/GAME/BP_Disk.BP_Disk_C|GetisInserted _disktoinsertref))
          (CallFunction|SimpleMailBoxInsert _disktoinsertref)
          (Utilities|FlowControl|Delay 0.2)
          ;[1 1 1] Small Delay as a security to prevent same disk to be inserted multiple times (OverlappComponent Triggered 3 times when disk is inserted)
          (Variables|DiskLogic|SetInsertionComplete true)
          (Variables|/Game/GAME/BP_Disk.BP_Disk_C|SetisInserted _disktoinsertref true))))))

(event Custom|StartWolfheadCheckLoop
  (Utilities|Time|SetTimerbyEvent (delegate Custom|StartWolfheadCheckLoop) 4e+02 true)
  (Development|PrintString "WOLFHEAD LOOP DELIVERY CHECK")
  (if (Utilities|Array|IsNotEmpty (Variables|Default|GetDiskSentToWolfhead))
    (Default|PlaySimpleSFX (Variables|Default|GetBP_AudioPlay) "/Game/GAME/AUDIO/SFX/SFX_Mailbox-Delivery.SFX_Mailbox-Delivery" "NewEnumerator1" (Transformation|GetWorldLocation (Variables|Default|GetAudio)) 1.0)
    (Utilities|FlowControl|Delay 3.5)
    (CallFunction|WolfheadDelivery)))

(event EventBeginPlay
  ;[0.3075 0.4947 1] BeginPlay
  (CallFunction|StartWolfheadCheckLoop))

(event EventTick
  (params (DeltaSeconds :type Float%20%28single-precision%29))
  ;[1 0.1869 0.2167] Event Tick
)

(event EventInteract
  (params (StaticMeshTouched :type Primitive%20Component%20Object%20Reference))
  (CallFunction|InteractFunction StaticMeshTouched))

(fn ConstructionScript)

(fn InteractFunction
  (params (StaticMeshTouched :type Primitive%20Component%20Object%20Reference))
  (bind _interactiontypeselecter (Default|GetInteractionType (Variables|Default|GetBP_StationInteraction) StaticMeshTouched))
  (switch Utilities|FlowControl|Switch|SwitchonE_InteractionType _interactiontypeselecter
    (:NewEnumerator10
      (CallFunction|LeverInteraction))
    (:NewEnumerator11
      (CallFunction|EjectMailboxContent))))

(fn LeverInteraction
  (bind _mailbox_lever (Variables|Default|GetMailBox_Lever))
  (bind _returnvalue (Transformation|GetWorldRotation _mailbox_lever))
  (Transformation|SetWorldRotation _mailbox_lever (Math|Rotator|MakeRotator (.roll _returnvalue) (Variables|Default|GetinteractedLeverRotation) (.yaw _returnvalue)) false false)
  (Default|PlaySimpleSFX (Variables|Default|GetBP_AudioPlay) "/Game/GAME/AUDIO/SFX/SFX_LeverDown.SFX_LeverDown" "NewEnumerator1" (Transformation|GetWorldLocation (Variables|Default|GetMailBox_Lever)) 1.0)
  (CallFunction|WolfheadCheck))

(fn EjectMailboxContent
  (Development|PrintString "Mail_Box Ejection")
  (if (Variables|DiskLogic|GetMailBoxFull)
    (Variables|DiskLogic|SetMailBoxFull false)
    (Default|PlaySimpleSFX (Variables|Default|GetBP_AudioPlay) "/Game/GAME/AUDIO/SFX/SFX_Mailbox-DiskEject.SFX_Mailbox-DiskEject" "NewEnumerator1" (Transformation|GetWorldLocation (Variables|Default|GetAudio)) 1.0)
    (for _array_element (Variables|DiskLogic|GetDiskInsideMailbox)
      (Default|MailBoxEjection _array_element self (Transformation|GetWorldLocation (Variables|Default|GetStartingDiskPoint))))))

(fn MailBoxInsertionSFX
  (if true
    (Default|PlaySimpleSFX (Variables|Default|GetBP_AudioPlay) "/Game/GAME/AUDIO/SFX/SFX_Mailbox-DiskInsert.SFX_Mailbox-DiskInsert" "NewEnumerator1" (Transformation|GetWorldLocation (Variables|Default|GetBox)) 1.0)))

(fn WolfheadCheck
  (for _array_element (Variables|DiskLogic|GetDiskInsideMailbox)
    (LocalVariables|SetcurrentDiskCheck _array_element)
    (switch string (.id (Variables|/Game/GAME/BP_Disk.BP_Disk_C|GetSignalDataInDisk _array_element))
      (:Default
        ;[1 1 1] Default Disk Empty Path
        (bind _diskvalid (WolfheadCheck|DiskEmptyCheck (LocalVariables|GetcurrentDiskCheck)))
        (if _diskvalid
          ;[1 1 1] Default Disk Processed Path
          (bind _diskvalid_2 (WolfheadCheck|DiskProcessCheck (LocalVariables|GetcurrentDiskCheck) false))
          (if _diskvalid_2
            ;[1 1 1] Default No Location Check
            (bind _diskvalid_3 (WolfheadCheck|DiskNoLocationCheck (LocalVariables|GetcurrentDiskCheck) false))
            (if (not _diskvalid_3)
              (CallFunction|DiskSenttoWolfheadSetup true (LocalVariables|GetcurrentDiskCheck)))
            (else
              (CallFunction|DiskSenttoWolfheadSetup true (LocalVariables|GetcurrentDiskCheck))))
          (else
            (CallFunction|DiskSenttoWolfheadSetup true (LocalVariables|GetcurrentDiskCheck)))))
      (:AD78B
        ;[1 1 1] Default Disk Empty Path
        (bind _diskvalid_4 (WolfheadCheck|DiskEmptyCheck (LocalVariables|GetcurrentDiskCheck)))
        (if _diskvalid_4
          ;[1 0.1651 0.1559] GIRL CRYING PROCESS OVERWRITE
          (bind _diskvalid_5 (WolfheadCheck|DiskProcessCheck (LocalVariables|GetcurrentDiskCheck) true "AHAH IS THAT A GIRL CRYING ??? "))
          (if _diskvalid_5
            ;[1 0.1651 0.1559] GIRL CRYIN LOCATION OVERWRITE
            (bind _diskvalid_6 (WolfheadCheck|DiskNoLocationCheck (LocalVariables|GetcurrentDiskCheck) false "\"I HAVE NO CARE IN HEARING A LITTLE GIRL CRYIN\""))
            (if _diskvalid_6
              ;[1 1 1] Default Wrong Location Check
              (bind _diskvalid_7 (WolfheadCheck|DiskWrongLocationCheck (LocalVariables|GetcurrentDiskCheck) "1789" true "WRONG LOCATION YOU RAT, DO YOUR JOB CORRECTLY"))
              (if _diskvalid_7
                (Development|PrintString "FUCKING HELL ITS A GOOD SPOT !" true true "(R=0.092016,G=1.000000,B=0.000000,A=1.000000)")
                (Default|EmptySignalData (LocalVariables|GetcurrentDiskCheck))
                (CallFunction|DiskSenttoWolfheadSetup false (LocalVariables|GetcurrentDiskCheck))
                ;[1 0.5268 0.376] (Temporary) Sucess
                (CallFunction|ModifyDiskText "NewEnumerator3" true "Good job !" (LocalVariables|GetcurrentDiskCheck))
                (else
                  (CallFunction|DiskSenttoWolfheadSetup true (LocalVariables|GetcurrentDiskCheck))))
              (else
                (CallFunction|DiskSenttoWolfheadSetup true (LocalVariables|GetcurrentDiskCheck))))
            (else
              (CallFunction|DiskSenttoWolfheadSetup true (LocalVariables|GetcurrentDiskCheck))))
          (else
            (CallFunction|DiskSenttoWolfheadSetup true (LocalVariables|GetcurrentDiskCheck)))))))
  ;[1 1 1] When we are done looping
  (Utilities|Array|Clear (Variables|DiskLogic|GetDiskInsideMailbox))
  (Variables|DiskLogic|SetMailBoxFull false))

(fn DiskEmptyCheck
  (params (disk :type BP%20Disk%20Object%20Reference))
  (if (Variables|/Game/GAME/BP_Disk.BP_Disk_C|GetisDiskEmpty disk)
    (CallFunction|ModifyDiskText "NewEnumerator0" false "" disk)
    (return false)
    (else
      (return true))))

(fn ModifyDiskText
  (params (commentType :type E_WolfheadResponseType%20Enum :default "NewEnumerator0") (overwriteDefaultComment :type Boolean) (wolfheadOverwriteTextComment :type String) (disk :type BP%20Disk%20Object%20Reference))
  (if overwriteDefaultComment
    (Default|SetWolfheadCommentText disk wolfheadOverwriteTextComment)
    (else
      (switch Utilities|FlowControl|Switch|SwitchonE_WolfheadResponseType commentType
        (:NewEnumerator0
          (Development|PrintString "DISK IS EMPTY YOU RAT")
          (Default|SetWolfheadCommentText disk "DISK IS EMPTY YOU RAT"))
        (:NewEnumerator1
          (Development|PrintString "CANT HEAR SHIT ! PROCESS IT ")
          (Default|SetWolfheadCommentText disk "CANT HEAR SHIT ! PROCESS IT "))
        (:NewEnumerator2
          (Development|PrintString "INTERESTING NOW DO YOUR  
JOB AND GIVE ME THE LOCATION")
          (Default|SetWolfheadCommentText disk "INTERESTING NOW DO YOUR  
JOB AND GIVE ME THE LOCATION"))
        (:NewEnumerator3
          (Development|PrintString "I CHECKED IT AND THERE IS NOTHING, I HOPE FOR YOU THAT IT WAS A LOCALSATION MISTAKE ! GIVE ME THE CORRECT LOCATION OF THAT SHIT ")
          (Default|SetWolfheadCommentText disk "I CHECKED IT AND THERE IS NOTHING, I HOPE FOR YOU THAT IT WAS A LOCALSATION MISTAKE ! GIVE ME THE CORRECT LOCATION OF THAT SHIT "))))))

(fn DiskProcessCheck
  (params (Disk :type BP%20Disk%20Object%20Reference) (overwriteWolfheadComment :type Boolean) (overwritingWolfheadText :type String))
  (if (.processed (Variables|/Game/GAME/BP_Disk.BP_Disk_C|GetSignalDataInDisk Disk))
    (return true)
    (else
      (CallFunction|ModifyDiskText "NewEnumerator1" overwriteWolfheadComment overwritingWolfheadText Disk)
      (return false))))

(fn DiskNoLocationCheck
  (params (Disk :type BP%20Disk%20Object%20Reference) (overwriteWolfheadComment :type Boolean) (overwritingWolfheadText :type String))
  (if (Utilities|Enum|Equal(Enum) (.localisation (Variables|/Game/GAME/BP_Disk.BP_Disk_C|GetSignalDataInDisk Disk)) "")
    (CallFunction|ModifyDiskText "NewEnumerator2" overwriteWolfheadComment overwritingWolfheadText Disk)
    (return false)
    (else
      (return true))))

(fn DiskWrongLocationCheck
  (params (Disk :type BP%20Disk%20Object%20Reference) (correctLocation :type String) (overwriteWolfheadComment :type Boolean) (overwritingWolfheadText :type String))
  (if (Utilities|Enum|NotEqual(Enum) (.localisation (Variables|/Game/GAME/BP_Disk.BP_Disk_C|GetSignalDataInDisk Disk)) correctLocation)
    (CallFunction|ModifyDiskText "NewEnumerator3" overwriteWolfheadComment overwritingWolfheadText Disk)
    (return false)
    (else
      (return true))))

(fn WolfheadDelivery
  (for _array_element (Variables|Default|GetDiskSentToWolfhead)
    (Default|MailBoxEjection _array_element self (Transformation|GetWorldLocation (Variables|Default|GetStartingDiskPoint))))
  (Utilities|Array|Clear (Variables|Default|GetDiskSentToWolfhead)))

(fn DiskSenttoWolfheadSetup
  (params (WolfheadNotHappy :type Boolean) (disk :type BP%20Disk%20Object%20Reference))
  (Variables|/Game/GAME/BP_Disk.BP_Disk_C|SetwolfheadNotHappyReject disk WolfheadNotHappy)
  (Utilities|Array|Add (Variables|Default|GetDiskSentToWolfhead) disk))

(fn SimpleMailBoxInsert
  (params (DiskInserted :type BP%20Disk%20Object%20Reference))
  (bind _endingdiskpoint (Variables|Default|GetEndingDiskPoint))
  (bind _returnvalue (Transformation|GetWorldLocation _endingdiskpoint))
  (Variables|DiskLogic|SetInsertionComplete false)
  (Sound|MailBoxInsertionSFX)
  (bind _output_get (Variables|DiskLogic|SetDiskRefBeingInserted DiskInserted))
  (Utilities|Array|Add (Variables|DiskLogic|GetDiskInsideMailbox) _output_get)
  (Variables|DiskLogic|SetMailBoxFull true)
  ;[1 1 1] DiskPosition
  (Transformation|SetWorldLocation (Actor|GetComponentbyClass (Variables|DiskLogic|GetDiskRefBeingInserted) "/Script/Engine.StaticMeshComponent") _returnvalue false false)
  (Transformation|SetActorLocation (Variables|DiskLogic|GetDiskRefBeingInserted) _returnvalue false false))