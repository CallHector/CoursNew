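; Short-range radio actor attached to the player for tuning into and homing in on nearby signal emitters.
; When enabled, mouse-wheel input changes frequency, and BPSignalScannerComponent looks up a matching signal, whose sound plays if active.
; A two-second timer loop compares emitter bearing to player facing by cardinal direction and scales signal volume by distance.
; It updates the character's scanner display and plays direction-dependent beeps within detection range, silencing them when very close.
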(event Custom|StartLoop
  ;[1 1 1] Start Loop
  (Utilities|Time|SetTimerbyEvent (delegate Custom|StartLoop) 2.0 true)
  (if (Variables|Default|GetradioEnabled)
    (if (Variables|Default|GetEmitterFound)
      ;[1 1 1] Signal Check Loop
      (CallFunction|SignalCheckLoop))))

(event Custom|MouseWheelUp
  (if (Variables|Default|GetlistenForMouseScrollInput)
    (CallFunction|FrequencyChanges 1.0)))

(event Custom|UpdateOrientationCorrect
  (params (isOrientationCorrect :type Boolean))
  ;[1 1 1] OrientationCorrect Scaner
  (Default|UpdateScannerInfo (Variables|Default|GetFirstPersonCharacter) false 0 false 0.0 "" false "" false isOrientationCorrect true))

(event Custom|MouseWheelDown
  (if (Variables|Default|GetlistenForMouseScrollInput)
    (CallFunction|FrequencyChanges -1.0)))

(event EventBeginPlay
  ;[0.2304 0.3524 1] BeginPlay
  (Transformation|AttachActorToActor (Game|GetPlayerCharacter 0) "None" "SnapToTarget" "SnapToTarget" "KeepRelative" true)
  (CallFunction|StartLoop)
  (bind _asbp_first_person_character (Utilities|Casting|CastToBP_FirstPersonCharacter (Game|GetPlayerCharacter 0))
    (:then
      (Variables|Default|SetFirstPersonCharacter _asbp_first_person_character))
    (:CastFailed
      (Development|PrintString "Error in BP_ProximitySignalScanner, the cast of the BP_FirstPersonCharacter Isn't working" true true "(R=1.000000,G=0.109946,B=0.000000,A=1.000000)"))))

(fn ConstructionScript)

(fn FrequencyChanges
  (params (isAdding :type Float%20%28double-precision%29))
  (bind _bp_signalscannercomponent (Variables|Default|GetBP_SignalScannerComponent))
  ;[1 0.7645 0.3118] SFX
  (Sound|FreqChangesSFX)
  ;[1 1 1] debug To see the frequency
  (Development|PrintString (Utilities|String|ToString(Float) (+ (Variables|/Game/GAME/ImportantsActors/BP_SignalScannerComponent.BP_SignalScannerComponent_C|GetscannerFrequency _bp_signalscannercomponent) (* (Variables|Default|GetfrequencyChangesAdd) isAdding))))
  (bind _output_get (Variables|/Game/GAME/ImportantsActors/BP_SignalScannerComponent.BP_SignalScannerComponent_C|SetscannerFrequency _bp_signalscannercomponent (+ (Variables|/Game/GAME/ImportantsActors/BP_SignalScannerComponent.BP_SignalScannerComponent_C|GetscannerFrequency _bp_signalscannercomponent) (* (Variables|Default|GetfrequencyChangesAdd) isAdding))))
  (bind (_signaldatafound _anysignaldatafound _numberofsignalfound _signaldatamultiple _actoremitting) (Default|SearchSignalProximityScanner (Variables|Default|GetBP_SignalScannerComponent) _output_get))
  (if _anysignaldatafound
    ;[1 1 1] Checking if signal is Active
    (if (.IsSignalActive (Utilities|Struct|BreakSignalDataStructure _signaldatafound))
      (Variables|Default|SetSignalDataTargeted _signaldatafound)
      (bind _output_get_2 (Variables|Default|SetActorEmitterTargeted _actoremitting))
      (Development|PrintString (Utilities|String|Append "ACTOR FOUND : " (Utilities|GetDisplayName _output_get_2)) true true "(R=1.000000,G=0.000000,B=0.199848,A=1.000000)")
      (Variables|Default|SetEmitterFound true)
      ;[1 1 1] Feedback SoundFound
      (Default|PlaySimpleSFX (Variables|Default|GetBP_AudioPlay) 0 "NewEnumerator6" (Transformation|GetWorldLocation (Variables|Default|GetAudio)) 1.0)
      (CallFunction|SetupSignal)
      (else
        (Variables|Default|SetEmitterFound false :!label _label)
        ;[1 1 1 1 15] Small Security to set the volume to 0 when changing frequency
        (CallFunction|AdjustSignalPlaying 0.0 true)
        ;[1 1 1 1 12] Small Secuirty to set the color of the scanner ro white when we change freq
        (CallFunction|UpdateOrientationCorrect false)))
    (else
      (goto _label)))
  ;[1 1 1 1 15] Player Scanner Freq Update
  (Default|UpdateRadioInfo (Variables|Default|GetFirstPersonCharacter) (Variables|/Game/GAME/ImportantsActors/BP_SignalScannerComponent.BP_SignalScannerComponent_C|GetscannerFrequency (Variables|Default|GetBP_SignalScannerComponent)) true (Variables|Default|GetEmitterFound) false "" false false false))

(fn BipSFX
  (params (bipType :type Integer))
  (LocalVariables|SetSoundPosition (Transformation|GetWorldLocation (Variables|/Script/Engine.Actor|GetRootComponent (Variables|Default|GetFirstPersonCharacter))))
  (switch int bipType
    (:0
      (Default|PlaySimpleSFX (Variables|Default|GetBP_AudioPlay) "/Game/GAME/AUDIO/SCANNER/SFX_Scan_Neutral.SFX_Scan_Neutral" "NewEnumerator1" (LocalVariables|GetSoundPosition) 1.0))
    (:1
      (Default|PlaySimpleSFX (Variables|Default|GetBP_AudioPlay) "/Game/GAME/AUDIO/SCANNER/SFX_Scan_Good1.SFX_Scan_Good1" "NewEnumerator1" (LocalVariables|GetSoundPosition) 1.0))
    (:2
      (Default|PlaySimpleSFX (Variables|Default|GetBP_AudioPlay) "/Game/GAME/AUDIO/SCANNER/SFX_Scan_Good2.SFX_Scan_Good2" "NewEnumerator1" (LocalVariables|GetSoundPosition) 1.0))
    (:3
      (Default|PlaySimpleSFX (Variables|Default|GetBP_AudioPlay) "/Game/GAME/AUDIO/SCANNER/SFX_Scan_Good3.SFX_Scan_Good3" "NewEnumerator1" (LocalVariables|GetSoundPosition) 1.0))))

(fn DistanceCheck
  (if (Variables|Default|GetEmitterFound)
    (return (/ (Math|Vector|VectorLength (- (Transformation|GetActorLocation (Variables|/Game/GAME/ImportantsActors/BP_SignalScannerComponent.BP_SignalScannerComponent_C|GetActorEmmitingFound (Variables|Default|GetBP_SignalScannerComponent))) (Transformation|GetWorldLocation (Variables|/Script/Engine.Character|GetCapsuleComponent (Game|GetPlayerCharacter 0))))) 1e+02))))

(fn ShowRadio
  (Variables|Default|SetradioEnabled true)
  (Development|PrintString "RadioEnabled")
  (Sound|ShowScannerSFX)
  (Default|ShowShortRangeRadio (Variables|Default|GetFirstPersonCharacter))
  (CallFunction|FrequencyChanges 0.0))

(fn HideRadio
  (Variables|Default|SetradioEnabled false)
  (Development|PrintString "RadioDisabled")
  (Sound|HideScannerSFX)
  (Default|HideShortRangeRAdio (Variables|Default|GetFirstPersonCharacter))
  (CallFunction|AdjustSignalPlaying 0.0 true))

(fn ListenforMouseScroll
  (params (listenForMouseScrollInput :type Boolean))
  (Variables|Default|SetlistenForMouseScrollInput listenForMouseScrollInput))

(fn FreqChangesSFX
  (Default|PlaySimpleSFX (Variables|Default|GetBP_AudioPlay) 0 "NewEnumerator2" (Transformation|GetWorldLocation (Variables|/Script/Engine.Character|GetCapsuleComponent (Game|GetPlayerCharacter 0))) 1.0))

(fn ShowScannerSFX
  (Default|PlaySimpleSFX (Variables|Default|GetBP_AudioPlay) "/Engine/VREditor/Sounds/UI/Floating_UI_Open-002.Floating_UI_Open-002" "NewEnumerator1" (Transformation|GetWorldLocation (Variables|/Script/Engine.Character|GetCapsuleComponent (Variables|Default|GetFirstPersonCharacter))) 1.0))

(fn HideScannerSFX
  (Default|PlaySimpleSFX (Variables|Default|GetBP_AudioPlay) "/Engine/VREditor/Sounds/UI/Floating_UI_Close-002.Floating_UI_Close-002" "NewEnumerator1" (Transformation|GetWorldLocation (Variables|/Script/Engine.Character|GetCapsuleComponent (Variables|Default|GetFirstPersonCharacter))) 1.0))

(fn AdjustSignalPlaying
  (params (distance :type Float%20%28double-precision%29) (disableSignal :type Boolean))
  (if disableSignal
    (Audio|Components|Audio|AdjustVolume (Variables|Default|GetAudio) 0.0 0.0 "Linear" :!class /Script/Engine.AudioComponent)
    (else
      (Audio|Components|Audio|AdjustVolume (Variables|Default|GetAudio) 0.0 (Math|Float|Lerp 0.7 0.0001 (/ (Math|Float|Clamp(Float) (- distance 1.0) 0.0 (Variables|Default|GetdistanceMinimumToHearSignal)) (Variables|Default|GetdistanceMinimumToHearSignal))) "Linear" :!class /Script/Engine.AudioComponent))))

(fn SetupSignal
  (bind _signaldatatargeted (Variables|Default|GetSignalDataTargeted))
  (Variables|Default|SetSignalDataPlaying _signaldatatargeted)
  (Audio|Components|Audio|SetSound (Variables|Default|GetAudio) (.sound (Utilities|Struct|BreakSignalDataStructure _signaldatatargeted)))
  (Audio|Components|Audio|Play (Variables|Default|GetAudio) 0.0)
  (Audio|Components|Audio|AdjustVolume (Variables|Default|GetAudio) 0.0 1e-05 "Linear" :!class /Script/Engine.AudioComponent))

(fn SignalCheckLoop
  (bind _distance (CallFunction|DistanceCheck))
  (LocalVariables|SetdistanceToSignal _distance)
  ;[1 0.6609 0.9011] Return Correct Orientation Or Not
  ;;[1 1 1] Player - Object Orientation
  (bind (_cardinaldirectionoutput _bearingnumbersoutput) (Default|ReturnBearingCardinalInfo (Variables|Default|GetBP_SignalScannerComponent) (Transformation|GetWorldLocation (Variables|/Script/Engine.Character|GetCapsuleComponent (Variables|Default|GetFirstPersonCharacter))) (Transformation|GetWorldLocation (Variables|/Game/GAME/BP_ItemTransmitting.BP_ItemTransmitting_C|GetStaticMesh (Variables|Default|GetActorEmitterTargeted)))))
  ;;[1 1 1] Player Camera Orientation
  (bind (_cardinaldirecton _bearingnumber) (Default|ReturnOrientation (Variables|Default|GetFirstPersonCharacter)))
  (bind _output_get (LocalVariables|SetOrientationCorrect (Utilities|Enum|Equal(Enum) _cardinaldirecton _cardinaldirectionoutput)))
  (CallFunction|UpdateOrientationCorrect _output_get)
  ;[1 1 1] Adjust Signal Playing
  (CallFunction|AdjustSignalPlaying (LocalVariables|GetdistanceToSignal) false)
  ;[1 1 1] Distance Check
  ;;[1 1 1 1 12] So Close that the Bip Stop and we hear the signal only
  (if (not (<= (LocalVariables|GetdistanceToSignal) (Variables|Default|GetdistanceStopBipNoise)))
    ;;[1 1 1 1 12] Close enough to have the Bip Sound?
    (if (<= (LocalVariables|GetdistanceToSignal) (Variables|Default|GetdistanceMinimumToHaveSignalDetection))
      (if (LocalVariables|GetOrientationCorrect)
        (CallFunction|BipSFX 1)
        (else
          (CallFunction|BipSFX))))))