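; Key item actor with a configurable static mesh and support for an inspection rotation query.
; On BeginPlay it applies StaticMeshSet to its StaticMesh component when that asset is valid.
; A Destroy event removes the actor after a short delay, and GetInspectRotation returns a zero rotation.
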(event Custom|Destroy
  (Utilities|FlowControl|Delay 0.2)
  (Actor|DestroyActor))

(event EventBeginPlay
  (if (Utilities|IsValid (Variables|StaticMesh|GetStaticMeshSet))
    (Components|StaticMesh|SetStaticMesh (Variables|Default|GetStaticMesh) (Variables|StaticMesh|GetStaticMeshSet))))

(fn ConstructionScript)

(fn GetInspectRotation
  (return "0, 0, 0"))