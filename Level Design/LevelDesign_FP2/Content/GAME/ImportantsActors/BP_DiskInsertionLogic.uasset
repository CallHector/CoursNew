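; BP_DiskInsertionLogic handles inserting a BP_Disk.
; IsInsertionValid accepts a disk only when its InsertionValidSecurity flag is set, then passes it to Insert.
; Insert interrupts the first-person character's grab, calls the disk's Insertion and stores the disk reference.
; A delayed custom event then sets ActivateDiskInsertion, while Eject is still an empty stub.
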(event Custom|InsertDelay
  (params (Delay :type Float%20%28double-precision%29))
  (Utilities|FlowControl|Delay Delay)
  (Variables|Default|SetActivateDiskInsertion true))

(fn Eject)

(fn Insert
  (params (DiskInserted :type BP%20Disk%20Object%20Reference))
  (bind _diskreference (CallFunction|InsertionGrabber DiskInserted))
  (Default|Insertion _diskreference)
  ;[1 1 1] Small Delay annoying but necessary I think?
  (CallFunction|InsertDelay (Variables|Default|GetInsertionDelay))
  (bind _output_get (Variables|Default|SetDiskToInsertRef DiskInserted))
  (Development|PrintString (Utilities|GetDisplayName _output_get)))

(fn InsertionGrabber
  (params (DiskToGrab :type BP%20Disk%20Object%20Reference))
  (bind _asbp_first_person_character (Utilities|Casting|CastToBP_FirstPersonCharacter (Game|GetPlayerCharacter 0))
    (:then
      (if (Variables|/Game/FirstPerson/Blueprints/BP_FirstPersonCharacter.BP_FirstPersonCharacter_C|GetisGrabbingObject _asbp_first_person_character)
        (Default|GrabInteruption _asbp_first_person_character)
        (return DiskToGrab)))
    (:CastFailed
      (Development|PrintString "Insertion Grabber : First Person Cast Failed"))))

(fn IsInsertionValid
  (params (ActorInserted :type Actor%20Object%20Reference))
  (bind _asbp_disk (Utilities|Casting|CastToBP_Disk ActorInserted))
  (if (== _asbp_disk ActorInserted)
    ;[1 1 1] Security To Prevent Insert when grabbing
    (if (Variables|/Game/GAME/BP_Disk.BP_Disk_C|GetInsertionValidSecurity _asbp_disk)
      (CallFunction|Insert _asbp_disk)
      (return true)
      (else
        _)))
  (return false))