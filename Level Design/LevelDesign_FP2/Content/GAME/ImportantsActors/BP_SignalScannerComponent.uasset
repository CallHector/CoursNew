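; Signal scanner component that finds in-world signal emitters by frequency or ID through the BPI_Signal interface.
; ModifyFrequency stores the tuned frequency and runs SearchSignal, which polls all emitters at whole-number steps across the filter band.
; Localisator search returns the first ID match, while proximity search returns the first exact-frequency match as a BP_ItemTransmitting.
; Standalone helpers convert origin and target positions into a compass bearing, eight-way cardinal direction and rounded distance in metres.
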(event EventBeginPlay)

(event EventTick
  (params (DeltaSeconds :type Float%20%28single-precision%29)))

(fn SearchSignal
  (params (frequencyScanned :type Float%20%28double-precision%29))
  (bind _signaldatafoundarray (Variables|SignalFound|GetsignalDataFoundArray))
  (bind _scannerfrequencyfilterband (Variables|Default|GetscannerFrequencyFilterBand))
  (bind _returnvalue (Utilities|Array|Length _signaldatafoundarray))
  (bind _returnvalue_2 (/ _scannerfrequencyfilterband 2.0))
  ;[1 1 1] To Improve to keep a sound playing
  (Utilities|Array|Clear (Variables|SignalFound|GetsignalDataFoundArray))
  (Variables|Default|SetIndex 0)
  ;[1 1 1] To prevent a Get All actors from interface on every loop
  (bind _outactors (Actor|GetAllActorswithInterface "/Game/GAME/ImportantsActors/BPI_Signal.BPI_Signal_C"))
  (Variables|Default|SetEmmittingSignalActors _outactors)
  (bind _index (Utilities|FlowControl|ForLoopwithBreak (Math|Float|Truncate (- frequencyScanned _returnvalue_2)) (Math|Float|Truncate (+ frequencyScanned _returnvalue_2)))
    (:LoopBody
      (for _array_element (Variables|Default|GetEmmittingSignalActors)
        (bind (_signaldata _found) (Class|BPISignal|FrequencyCheck(Message) _array_element (Math|Conversions|ToFloat(Integer) _index)))
        (if _found
          (Utilities|Array|SetArrayElem (Variables|SignalFound|GetsignalDataFoundArray) (Variables|Default|GetIndex) _signaldata true)
          (Variables|Default|SetIndex (+ (Variables|Default|GetIndex) 1)))))
    (:Completed
      (return "" (> _returnvalue 0) _returnvalue _signaldatafoundarray))))

(fn ModifyFrequency
  (params (frequencyChanges :type Float%20%28double-precision%29))
  (bind _output_get (Variables|Default|SetscannerFrequency frequencyChanges))
  (bind (_signaldatafound _anysignaldatafound _numberofsignalfound _signaldatamultiple) (CallFunction|SearchSignal _output_get))
  (for _index (range 0 (Utilities|Array|Length _signaldatamultiple))
    ;[1 1 1] Condition to know if we found a signal or not
    (if (> (Utilities|Array|Length _signaldatamultiple) 0)
      (Development|PrintString (Utilities|String|Append "Signal ID found : " (.ID (Utilities|Struct|BreakSignalDataStructure (Utilities|Array|Get(acopy) _signaldatamultiple _index)))))
      (return _signaldatamultiple _anysignaldatafound))))

(fn SearchSignalLocalisator
  (params (ID :type String))
  ;[1 1 1] To prevent a Get All actors from interface on every loop
  (bind _outactors (Actor|GetAllActorswithInterface "/Game/GAME/ImportantsActors/BPI_Signal.BPI_Signal_C"))
  (bind _output_get (Variables|Default|SetEmmittingSignalActors _outactors))
  (for _array_element _output_get
    (bind (_signaldata _found) (Class|BPISignal|IDCheck(Message) _array_element ID))
    (if _found
      (Variables|Default|SetActorEmmitingFound 0)
      (return _signaldata true 0 0 _array_element)))
  (return "" false 0 0 0))

(fn SearchSignalProximityScanner
  (params (Frequency :type Float%20%28double-precision%29))
  ;[1 1 1] To prevent a Get All actors from interface on every loop
  (bind _outactors (Actor|GetAllActorswithInterface "/Game/GAME/ImportantsActors/BPI_Signal.BPI_Signal_C"))
  (bind _output_get (Variables|Default|SetEmmittingSignalActors _outactors))
  (for _array_element _output_get
    (bind (_signaldata _found) (Class|BPISignal|FrequencyCheck(Message) _array_element Frequency))
    (if _found
      (bind _asbp_item_transmitting (Utilities|Casting|CastToBP_ItemTransmitting _array_element))
      (bind _output_get_2 (Variables|Default|SetActorEmmitingFound _asbp_item_transmitting))
      (return _signaldata true 0 0 _output_get_2)))
  (return "" false 0 0 0))

(fn ReturnBearingCardinalInfo
  (params (origin :type Vector) (target :type Vector))
  (bind _returnvalue (- target origin))
  (bind _returnvalue_2 (Math|Rotator|MakeRotfromX _returnvalue))
  (bind _returnvalue_3 (+ (.yaw _returnvalue_2) 3.6e+02))
  (if (< (.yaw _returnvalue_2) 0.0)
    (LocalVariables|SetBearingNumbers (Math|Float|Round _returnvalue_3))
    (LocalVariables|SetCardinalNumber (Math|Integer|%(Integer) (Math|Float|Floor (/ _returnvalue_3 45.0)) 8))
    (else
      (LocalVariables|SetBearingNumbers (Math|Float|Round (.yaw _returnvalue_2)))
      (LocalVariables|SetCardinalNumber (Math|Integer|%(Integer) (Math|Float|Floor (/ (.yaw _returnvalue_2) 45.0)) 8))))
  (switch int (LocalVariables|GetCardinalNumber)
    (:0
      (return "NewEnumerator0" (LocalVariables|GetBearingNumbers)))
    (:1
      (return "NewEnumerator5" (LocalVariables|GetBearingNumbers)))
    (:2
      (return "NewEnumerator2" (LocalVariables|GetBearingNumbers)))
    (:3
      (return "NewEnumerator7" (LocalVariables|GetBearingNumbers)))
    (:4
      (return "NewEnumerator3" (LocalVariables|GetBearingNumbers)))
    (:5
      (return "NewEnumerator6" (LocalVariables|GetBearingNumbers)))
    (:6
      (return "NewEnumerator1" (LocalVariables|GetBearingNumbers)))
    (:7
      (return "NewEnumerator4" (LocalVariables|GetBearingNumbers)))))

(fn ReturnDistanceInfo
  (params (origin :type Vector) (target :type Vector))
  (return (Math|Float|Round (/ (Math|Vector|VectorLength (- origin target)) 1e+02))))