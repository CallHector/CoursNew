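; BP_AudioPlay is an audio helper that plays signal sounds, generic interaction SFX and one controllable tracked sound.
; Signal and SFX calls play one-shots at a location, with an enum mapping generic types to preset sounds, which, unlike passed-in sounds, get no attenuation settings.
; Tracked playback stores a supplied AudioComponent for stop, pause and resume.
; IsPlaying is set by signal and tracked playback and cleared only by stopping.
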(event EventBeginPlay)

(event EventTick
  (params (DeltaSeconds :type Float%20%28single-precision%29)))

(fn PlaySimpleSignalAudio
  (params (SignalData :type Signal%20Data%20Structure%20Structure) (AudioPosition :type Vector))
  (Audio|PlaySoundatLocation (.sound (Utilities|Struct|BreakSignalDataStructure SignalData)) AudioPosition "0, 0, 0" 1.0 1.0 0.0 "/Game/GAME/SND_ATTENUATION.SND_ATTENUATION" 0 0 0)
  (Variables|Default|SetisPlaying true))

(fn StopTrackedAudio
  (Audio|Components|Audio|Stop (Variables|Default|GetaudioComponentTracked))
  (Variables|Default|SetisPlaying false))

(fn PlayTrackedAudio
  (params (soundToPlay :type Sound%20Base%20Object%20Reference) (AudioComponentToTrack :type Audio%20Component%20Object%20Reference) (startTime :type Float%20%28double-precision%29))
  (bind _output_get (Variables|Default|SetaudioComponentTracked AudioComponentToTrack))
  (Transformation|AttachComponentToComponent _output_get 0 "None" "KeepRelative" "KeepRelative" "KeepRelative" true)
  (Audio|Components|Audio|SetSound _output_get soundToPlay)
  (Audio|Components|Audio|Play _output_get startTime)
  (Variables|Default|SetisPlaying true))

(fn PauseTrackedAudio
  (Class|AudioComponent|SetPaused (Variables|Default|GetaudioComponentTracked) true))

(fn ResumeTrackedAudio
  (Class|AudioComponent|SetPaused (Variables|Default|GetaudioComponentTracked) false))

(fn PlaySimpleSFX
  (params (SoundToPlay :type Sound%20Base%20Object%20Reference) (GenericSoundType :type E_GenericSoundType%20Enum :default "NewEnumerator0") (Position :type Vector) (volumeMultiplier :type Float%20%28double-precision%29))
  (LocalVariables|SetPositionOfSFX Position)
  (LocalVariables|SetLocalVolumeMultiplier volumeMultiplier)
  (if (Utilities|Enum|Equal(Enum) GenericSoundType "NewEnumerator1")
    (Audio|PlaySoundatLocation SoundToPlay Position "0, 0, 0" (LocalVariables|GetLocalVolumeMultiplier) 1.0 0.0 "/Game/GAME/SND_ATTENUATION.SND_ATTENUATION" 0 0 0)
    (else
      (switch Utilities|FlowControl|Switch|SwitchonE_GenericSoundType GenericSoundType
        (:NewEnumerator2
          (Audio|PlaySoundatLocation "/Game/GAME/AUDIO/SFX/SFX_Radio_FrequencyChange.SFX_Radio_FrequencyChange" (LocalVariables|GetPositionOfSFX) "0, 0, 0" (LocalVariables|GetLocalVolumeMultiplier) 1.0 0.0 "/Game/GAME/SND_ATTENUATION.SND_ATTENUATION" 0 0 0))
        (:NewEnumerator3
          (Audio|PlaySoundatLocation "/Engine/VREditor/Sounds/VR_click1_Cue.VR_click1_Cue" (LocalVariables|GetPositionOfSFX) "0, 0, 0" (LocalVariables|GetLocalVolumeMultiplier) 1.0 0.0 "/Game/GAME/SND_ATTENUATION.SND_ATTENUATION" 0 0 0))
        (:NewEnumerator4
          (Audio|PlaySoundatLocation "/Engine/VREditor/Sounds/UI/Invalid_Action.Invalid_Action" (LocalVariables|GetPositionOfSFX) "0, 0, 0" (LocalVariables|GetLocalVolumeMultiplier) 1.0 0.0 "/Game/GAME/SND_ATTENUATION.SND_ATTENUATION" 0 0 0))
        (:NewEnumerator5
          (Audio|PlaySoundatLocation "/Engine/VREditor/Sounds/UI/Dockable_Window_Drop.Dockable_Window_Drop" (LocalVariables|GetPositionOfSFX) "0, 0, 0" (LocalVariables|GetLocalVolumeMultiplier) 1.0 0.0 "/Game/GAME/SND_ATTENUATION.SND_ATTENUATION" 0 0 0))
        (:NewEnumerator6
          (Audio|PlaySoundatLocation "/Engine/EditorSounds/Notifications/CompileStart_Cue.CompileStart_Cue" (LocalVariables|GetPositionOfSFX) "0, 0, 0" (LocalVariables|GetLocalVolumeMultiplier) 1.0 0.0 "/Game/GAME/SND_ATTENUATION.SND_ATTENUATION" 0 0 0))
        (:NewEnumerator7
          (Audio|PlaySoundatLocation "/Engine/EditorSounds/Notifications/CompileSuccess_Cue.CompileSuccess_Cue" (LocalVariables|GetPositionOfSFX) "0, 0, 0" (LocalVariables|GetLocalVolumeMultiplier) 1.0 0.0 "/Game/GAME/SND_ATTENUATION.SND_ATTENUATION" 0 0 0))
        (:NewEnumerator8
          ;[1 1 1] Used By BP_Radio Record Valid and Pressed
          (Audio|PlaySoundatLocation "/Engine/VREditor/Sounds/UI/Click_on_Button_Cue.Click_on_Button_Cue" (LocalVariables|GetPositionOfSFX) "0, 0, 0" (LocalVariables|GetLocalVolumeMultiplier) 1.0 0.0 "/Game/GAME/SND_ATTENUATION.SND_ATTENUATION" 0 0 0))
        (:NewEnumerator9
          ;[1 1 1] Used bY
          (Audio|PlaySoundatLocation "/Engine/VREditor/Sounds/UI/Dockable_Window_Open.Dockable_Window_Open" (LocalVariables|GetPositionOfSFX) "0, 0, 0" (LocalVariables|GetLocalVolumeMultiplier) 1.0 0.0 "/Game/GAME/SND_ATTENUATION.SND_ATTENUATION" 0 0 0))
        (:NewEnumerator10
          ;[1 1 1] Used By BP_Radio Record Ready
          (Audio|PlaySoundatLocation "/Engine/VREditor/Sounds/UI/Object_Snaps_To_Grid.Object_Snaps_To_Grid" (LocalVariables|GetPositionOfSFX) "0, 0, 0" (LocalVariables|GetLocalVolumeMultiplier) 1.0 0.0 "/Game/GAME/SND_ATTENUATION.SND_ATTENUATION" 0 0 0))
        (:NewEnumerator11
          (Audio|PlaySoundatLocation "/Engine/VREditor/Sounds/UI/Object_Snaps_To_Another_Actor.Object_Snaps_To_Another_Actor" (LocalVariables|GetPositionOfSFX) "0, 0, 0" (LocalVariables|GetLocalVolumeMultiplier) 1.0 0.0 "/Game/GAME/SND_ATTENUATION.SND_ATTENUATION" 0 0 0))
        (:NewEnumerator12
          (Audio|PlaySoundatLocation "/Game/GAME/AUDIO/SFX/SFX_Keyboard-SpaceBar.SFX_Keyboard-SpaceBar" (LocalVariables|GetPositionOfSFX) "0, 0, 0" (LocalVariables|GetLocalVolumeMultiplier) 1.0 0.0 "/Game/GAME/SND_ATTENUATION.SND_ATTENUATION" 0 0 0))))))