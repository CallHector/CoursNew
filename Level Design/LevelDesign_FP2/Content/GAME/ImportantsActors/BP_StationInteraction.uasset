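; BP_StationInteraction classifies which piece of station equipment was touched, such as keyboard, processor, localisator, radio, recorder or mail box controls.
; GetInteractionType derives a name from the touched static mesh's object name by chopping the string, then switches on it to return an interaction-type enum.
; Related parts share one type, and unknown names fall back to a default.
; The event graph is empty, and disconnected debug prints remain in the function.
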(event EventBeginPlay)

(event EventTick
  (params (DeltaSeconds :type Float%20%28single-precision%29)))

(fn GetInteractionType
  (params (StaticMeshTouched :type Primitive%20Component%20Object%20Reference))
  (bind _returnvalue (Utilities|GetObjectName StaticMeshTouched))
  (bind _output_get (Variables|Default|SetstaticMeshName (Utilities|String|RightChop _returnvalue (+ (Utilities|String|FindSubstring _returnvalue " ") 1))))
  (switch string _output_get
    (:Default
      (return "NewEnumerator4"))
    (:KEYBOARD
      (return "NewEnumerator0"))
    (:LOCALISATOR_SCREEN
      _)
    (:LOCALISATOR
      _)
    (:COMPUTER_DISK
      (return "NewEnumerator1"))
    (:PROCESSOR
      (return "NewEnumerator8"))
    (:PROCESSOR_SCREEN
      (return "NewEnumerator8"))
    (:SignalRecordScreen
      ;[1 1 1] Old
      (return "NewEnumerator6"))
    (:ComputerTower
      (return "NewEnumerator1"))
    (:HIFI_Processor
      (return "NewEnumerator1"))
    (:HIFI_Localisator
      (return "NewEnumerator1"))
    (:Computer_Extractor
      (return "NewEnumerator7"))
    (:MailBox_Lever
      (return "NewEnumerator10"))
    (:MailBox_ButtonEject
      (return "NewEnumerator11"))
    (:RadioSwitch
      (return "NewEnumerator5"))
    (:RadioRecorder
      (return "NewEnumerator12"))
    (:Voltmeter
      (return "NewEnumerator5"))
    (:FrequencyRadio
      (return "NewEnumerator5"))
    (:RecorderStaticMesh
      (return "NewEnumerator12")))
  (return "NewEnumerator9"))