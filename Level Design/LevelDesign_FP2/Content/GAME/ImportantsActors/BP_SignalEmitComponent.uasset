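; BP_SignalEmitComponent is a component that holds one signal's data and makes it available for lookup.
; GetDataFromFrequency returns the stored SignalData with a found flag when the given frequency exactly matches its SignalFrequency.
; GetDataFromID does the same by comparing the given SignalID to the data's ID, and both report not found on a mismatch.
; The event graph is empty, so it only answers queries.
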(event EventBeginPlay)

(event EventTick
  (params (DeltaSeconds :type Float%20%28single-precision%29)))

(fn GetDatafromFrequency
  (params (frequency :type Float%20%28double-precision%29))
  (bind _signaldata (Variables|Default|GetsignalData))
  (if (== (.signalFrequency (Utilities|Struct|BreakSignalDataStructure _signaldata)) frequency)
    (return _signaldata true)
    (else
      (return "" false))))

(fn GetDatafromID
  (params (signalID :type String))
  (bind _signaldata (Variables|Default|GetsignalData))
  (if (Utilities|Enum|Equal(Enum) signalID (.ID (Utilities|Struct|BreakSignalDataStructure _signaldata)))
    (return _signaldata true)
    (else
      (return "" false))))