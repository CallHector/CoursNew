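; Time-of-day manager that switches the level's lighting and atmosphere between Day, Night, Dusk and Red Night presets.
; BeginPlay applies DefaultTimeOfDay through ChangeTimeOfDay, which instantly toggles visibility of pre-placed sky sphere, directional light, skylight and height fog actors, with no blending.
; Red Night has its own skylight, while Night hides both fogs and also sets skylight intensity.
; Disconnected nodes for recoloring the day sky and skylight never run.
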(event EventBeginPlay
  (CallFunction|ChangeTimeOfDay (Variables|Default|GetdefaultTimeOfDay)))

(event Collision|EventActorBeginOverlap
  (params (OtherActor :type Actor%20Object%20Reference)))

(event EventTick
  (params (DeltaSeconds :type Float%20%28single-precision%29)))

(fn ConstructionScript)

(fn ChangeTimeOfDay
  (params (NewTimeOfDay :type E_TimeOfDay%20Enum :default "NewEnumerator0"))
  (switch Utilities|FlowControl|Switch|SwitchonE_TimeOfDay NewTimeOfDay
    (:NewEnumerator0
      ;[0.9219 0.9219 0.9219] DAY
      ;;[1 1 1] Sky Sphere
      (Rendering|SetActorHiddenInGame (Variables|SkySphere|GetDay_SkySphere) false)
      (Rendering|SetActorHiddenInGame (Variables|SkySphere|GetDusk_SkySphere) true)
      (Rendering|SetActorHiddenInGame (Variables|SkySphere|GetRedNight_SkySphere) true)
      (Rendering|SetActorHiddenInGame (Variables|SkySphere|GetNight_SkySphere) true)
      ;;[1 1 1] Directionnal Light
      (Rendering|SetActorHiddenInGame (Variables|DirectionnalLight|GetDay_DirectionnalLight) false)
      (Rendering|SetActorHiddenInGame (Variables|DirectionnalLight|GetDusk_DirectionnalLight) true)
      (Rendering|SetActorHiddenInGame (Variables|DirectionnalLight|GetRedNight_DirectionnalLight) true)
      (Rendering|SetActorHiddenInGame (Variables|DirectionnalLight|GetNight_DirectionnalLight) true)
      ;;[1 1 1] Sky Light
      (Rendering|SetActorHiddenInGame (Variables|SkyLight|GetSkyLight) false)
      (Rendering|SetActorHiddenInGame (Variables|SkyLight|GetRedNight_SkyLight) true)
      ;;[1 1 1] Exponential Height Fog
      (Rendering|SetActorHiddenInGame (Variables|ExponentialHeightFog|GetExponentialHeightFog) false)
      (Rendering|SetActorHiddenInGame (Variables|ExponentialHeightFog|GetDusk_ExponentialHeightFog) true))
    (:NewEnumerator1
      ;[0 0 0] DAY
      ;;[1 1 1] Sky Sphere
      (Rendering|SetActorHiddenInGame (Variables|SkySphere|GetDay_SkySphere) true)
      (Rendering|SetActorHiddenInGame (Variables|SkySphere|GetDusk_SkySphere) true)
      (Rendering|SetActorHiddenInGame (Variables|SkySphere|GetRedNight_SkySphere) true)
      (Rendering|SetActorHiddenInGame (Variables|SkySphere|GetNight_SkySphere) false)
      ;;[1 1 1] Directionnal Light
      (Rendering|SetActorHiddenInGame (Variables|DirectionnalLight|GetDay_DirectionnalLight) true)
      (Rendering|SetActorHiddenInGame (Variables|DirectionnalLight|GetDusk_DirectionnalLight) true)
      (Rendering|SetActorHiddenInGame (Variables|DirectionnalLight|GetRedNight_DirectionnalLight) true)
      (Rendering|SetActorHiddenInGame (Variables|DirectionnalLight|GetNight_DirectionnalLight) false)
      ;;[1 1 1] Sky Light
      (Rendering|SetActorHiddenInGame (Variables|SkyLight|GetSkyLight) false)
      (Rendering|SetActorHiddenInGame (Variables|SkyLight|GetRedNight_SkyLight) true)
      ;;[1 1 1] Exponential Height Fog
      (Rendering|SetActorHiddenInGame (Variables|ExponentialHeightFog|GetExponentialHeightFog) true)
      (Rendering|SetActorHiddenInGame (Variables|ExponentialHeightFog|GetDusk_ExponentialHeightFog) true)
      (Rendering|Components|Light|SetIntensity (Variables|/Script/Engine.SkyLight|GetLightComponent (Variables|SkyLight|GetSkyLight)) 1.0))
    (:NewEnumerator2
      ;[0.9219 0.6661 0.1583] DUSK
      ;;[1 1 1] Sky Sphere
      (Rendering|SetActorHiddenInGame (Variables|SkySphere|GetDay_SkySphere) true)
      (Rendering|SetActorHiddenInGame (Variables|SkySphere|GetDusk_SkySphere) false)
      (Rendering|SetActorHiddenInGame (Variables|SkySphere|GetRedNight_SkySphere) true)
      (Rendering|SetActorHiddenInGame (Variables|SkySphere|GetNight_SkySphere) true)
      ;;[1 1 1] Directionnal Light
      (Rendering|SetActorHiddenInGame (Variables|DirectionnalLight|GetDay_DirectionnalLight) true)
      (Rendering|SetActorHiddenInGame (Variables|DirectionnalLight|GetDusk_DirectionnalLight) false)
      (Rendering|SetActorHiddenInGame (Variables|DirectionnalLight|GetRedNight_DirectionnalLight) true)
      (Rendering|SetActorHiddenInGame (Variables|DirectionnalLight|GetNight_DirectionnalLight) true)
      ;;[1 1 1] Sky Light
      (Rendering|SetActorHiddenInGame (Variables|SkyLight|GetSkyLight) false)
      (Rendering|SetActorHiddenInGame (Variables|SkyLight|GetRedNight_SkyLight) true)
      ;;[1 1 1] Exponential Height Fog
      (Rendering|SetActorHiddenInGame (Variables|ExponentialHeightFog|GetExponentialHeightFog) true)
      (Rendering|SetActorHiddenInGame (Variables|ExponentialHeightFog|GetDusk_ExponentialHeightFog) false))
    (:NewEnumerator3
      ;[0.1559 0 0] RED NIGHT
      ;;[1 1 1] Sky Sphere
      (Rendering|SetActorHiddenInGame (Variables|SkySphere|GetDay_SkySphere) true)
      (Rendering|SetActorHiddenInGame (Variables|SkySphere|GetDusk_SkySphere) true)
      (Rendering|SetActorHiddenInGame (Variables|SkySphere|GetRedNight_SkySphere) false)
      (Rendering|SetActorHiddenInGame (Variables|SkySphere|GetNight_SkySphere) true)
      ;;[1 1 1] Directionnal Light
      (Rendering|SetActorHiddenInGame (Variables|DirectionnalLight|GetDay_DirectionnalLight) true)
      (Rendering|SetActorHiddenInGame (Variables|DirectionnalLight|GetDusk_DirectionnalLight) true)
      (Rendering|SetActorHiddenInGame (Variables|DirectionnalLight|GetRedNight_DirectionnalLight) false)
      (Rendering|SetActorHiddenInGame (Variables|DirectionnalLight|GetNight_DirectionnalLight) true)
      ;;[1 1 1] Sky Light
      (Rendering|SetActorHiddenInGame (Variables|SkyLight|GetSkyLight) true)
      (Rendering|SetActorHiddenInGame (Variables|SkyLight|GetRedNight_SkyLight) false)
      ;;[1 1 1] Exponential Height Fog
      (Rendering|SetActorHiddenInGame (Variables|ExponentialHeightFog|GetExponentialHeightFog) false)
      (Rendering|SetActorHiddenInGame (Variables|ExponentialHeightFog|GetDusk_ExponentialHeightFog) true))))