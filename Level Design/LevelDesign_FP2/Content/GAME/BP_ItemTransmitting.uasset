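; Item actor that transmits a signal through its BPSignalEmitComponent, with an optional mesh override applied at BeginPlay.
; SetSignalActive and SetSignalInactive rebuild the component's SignalData struct with one boolean flipped, keeping all other fields.
; FrequencyCheck and IDCheck forward lookups to the component, returning the signal data and a found flag.
; Interact only prints a debug string, and Destroy removes the actor after a short delay.
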(event Custom|Destroy
  (Utilities|FlowControl|Delay 0.2)
  (Actor|DestroyActor))

(event EventBeginPlay
  (if (Utilities|IsValid (Variables|StaticMesh|GetStaticMeshSet))
    (Components|StaticMesh|SetStaticMesh (Variables|Default|GetStaticMesh) (Variables|StaticMesh|GetStaticMeshSet))))

(fn ConstructionScript)

(fn Interact
  (Development|PrintString "Interaction Enabled"))

(fn SetSignalActive
  (bind _bp_signalemitcomponent (Variables|Default|GetBP_SignalEmitComponent))
  (Variables|/Game/GAME/ImportantsActors/BP_SignalEmitComponent.BP_SignalEmitComponent_C|SetsignalData _bp_signalemitcomponent (Utilities|Struct|MakeSignalDataStructure (.id (Variables|/Game/GAME/ImportantsActors/BP_SignalEmitComponent.BP_SignalEmitComponent_C|GetsignalData _bp_signalemitcomponent)) (.signalfrequency (Variables|/Game/GAME/ImportantsActors/BP_SignalEmitComponent.BP_SignalEmitComponent_C|GetsignalData _bp_signalemitcomponent)) (.sound (Variables|/Game/GAME/ImportantsActors/BP_SignalEmitComponent.BP_SignalEmitComponent_C|GetsignalData _bp_signalemitcomponent)) true (.firstrecord (Variables|/Game/GAME/ImportantsActors/BP_SignalEmitComponent.BP_SignalEmitComponent_C|GetsignalData _bp_signalemitcomponent)) (.firstinsert (Variables|/Game/GAME/ImportantsActors/BP_SignalEmitComponent.BP_SignalEmitComponent_C|GetsignalData _bp_signalemitcomponent)) (.firstprocess (Variables|/Game/GAME/ImportantsActors/BP_SignalEmitComponent.BP_SignalEmitComponent_C|GetsignalData _bp_signalemitcomponent)) (.newrecord (Variables|/Game/GAME/ImportantsActors/BP_SignalEmitComponent.BP_SignalEmitComponent_C|GetsignalData _bp_signalemitcomponent)) (.timeofrecord (Variables|/Game/GAME/ImportantsActors/BP_SignalEmitComponent.BP_SignalEmitComponent_C|GetsignalData _bp_signalemitcomponent)) (.startsoundtimeofrecord (Variables|/Game/GAME/ImportantsActors/BP_SignalEmitComponent.BP_SignalEmitComponent_C|GetsignalData _bp_signalemitcomponent)) (.localisation (Variables|/Game/GAME/ImportantsActors/BP_SignalEmitComponent.BP_SignalEmitComponent_C|GetsignalData _bp_signalemitcomponent)) (.processed (Variables|/Game/GAME/ImportantsActors/BP_SignalEmitComponent.BP_SignalEmitComponent_C|GetsignalData _bp_signalemitcomponent)) (.signalstrenght (Variables|/Game/GAME/ImportantsActors/BP_SignalEmitComponent.BP_SignalEmitComponent_C|GetsignalData _bp_signalemitcomponent)) (.signalaccuracy (Variables|/Game/GAME/ImportantsActors/BP_SignalEmitComponent.BP_SignalEmitComponent_C|GetsignalData _bp_signalemitcomponent)) (.processedsound (Variables|/Game/GAME/ImportantsActors/BP_SignalEmitComponent.BP_SignalEmitComponent_C|GetsignalData _bp_signalemitcomponent)) (.id_dev (Variables|/Game/GAME/ImportantsActors/BP_SignalEmitComponent.BP_SignalEmitComponent_C|GetsignalData _bp_signalemitcomponent)) (.localisation_dev (Variables|/Game/GAME/ImportantsActors/BP_SignalEmitComponent.BP_SignalEmitComponent_C|GetsignalData _bp_signalemitcomponent)) (.jammer (Variables|/Game/GAME/ImportantsActors/BP_SignalEmitComponent.BP_SignalEmitComponent_C|GetsignalData _bp_signalemitcomponent)))))

(fn SetSignalInactive
  (bind _bp_signalemitcomponent (Variables|Default|GetBP_SignalEmitComponent))
  (Variables|/Game/GAME/ImportantsActors/BP_SignalEmitComponent.BP_SignalEmitComponent_C|SetsignalData _bp_signalemitcomponent (Utilities|Struct|MakeSignalDataStructure (.id (Variables|/Game/GAME/ImportantsActors/BP_SignalEmitComponent.BP_SignalEmitComponent_C|GetsignalData _bp_signalemitcomponent)) (.signalfrequency (Variables|/Game/GAME/ImportantsActors/BP_SignalEmitComponent.BP_SignalEmitComponent_C|GetsignalData _bp_signalemitcomponent)) (.sound (Variables|/Game/GAME/ImportantsActors/BP_SignalEmitComponent.BP_SignalEmitComponent_C|GetsignalData _bp_signalemitcomponent)) false (.firstrecord (Variables|/Game/GAME/ImportantsActors/BP_SignalEmitComponent.BP_SignalEmitComponent_C|GetsignalData _bp_signalemitcomponent)) (.firstinsert (Variables|/Game/GAME/ImportantsActors/BP_SignalEmitComponent.BP_SignalEmitComponent_C|GetsignalData _bp_signalemitcomponent)) (.firstprocess (Variables|/Game/GAME/ImportantsActors/BP_SignalEmitComponent.BP_SignalEmitComponent_C|GetsignalData _bp_signalemitcomponent)) (.newrecord (Variables|/Game/GAME/ImportantsActors/BP_SignalEmitComponent.BP_SignalEmitComponent_C|GetsignalData _bp_signalemitcomponent)) (.timeofrecord (Variables|/Game/GAME/ImportantsActors/BP_SignalEmitComponent.BP_SignalEmitComponent_C|GetsignalData _bp_signalemitcomponent)) (.startsoundtimeofrecord (Variables|/Game/GAME/ImportantsActors/BP_SignalEmitComponent.BP_SignalEmitComponent_C|GetsignalData _bp_signalemitcomponent)) (.localisation (Variables|/Game/GAME/ImportantsActors/BP_SignalEmitComponent.BP_SignalEmitComponent_C|GetsignalData _bp_signalemitcomponent)) (.processed (Variables|/Game/GAME/ImportantsActors/BP_SignalEmitComponent.BP_SignalEmitComponent_C|GetsignalData _bp_signalemitcomponent)) (.signalstrenght (Variables|/Game/GAME/ImportantsActors/BP_SignalEmitComponent.BP_SignalEmitComponent_C|GetsignalData _bp_signalemitcomponent)) (.signalaccuracy (Variables|/Game/GAME/ImportantsActors/BP_SignalEmitComponent.BP_SignalEmitComponent_C|GetsignalData _bp_signalemitcomponent)) (.processedsound (Variables|/Game/GAME/ImportantsActors/BP_SignalEmitComponent.BP_SignalEmitComponent_C|GetsignalData _bp_signalemitcomponent)) (.id_dev (Variables|/Game/GAME/ImportantsActors/BP_SignalEmitComponent.BP_SignalEmitComponent_C|GetsignalData _bp_signalemitcomponent)) (.localisation_dev (Variables|/Game/GAME/ImportantsActors/BP_SignalEmitComponent.BP_SignalEmitComponent_C|GetsignalData _bp_signalemitcomponent)) (.jammer (Variables|/Game/GAME/ImportantsActors/BP_SignalEmitComponent.BP_SignalEmitComponent_C|GetsignalData _bp_signalemitcomponent)))))

(fn FrequencyCheck
  (params (frequency :type Float%20%28double-precision%29))
  (bind (_signaldata _signalfound) (Default|GetDatafromFrequency (Variables|Default|GetBP_SignalEmitComponent) frequency))
  (return _signaldata _signalfound))

(fn IDCheck
  (params (ID :type String))
  (bind (_signaldata _signalfound) (Default|GetDatafromID (Variables|Default|GetBP_SignalEmitComponent) ID))
  (return _signaldata _signalfound))